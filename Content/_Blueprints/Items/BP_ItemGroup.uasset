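; BP_ItemGroup is an actor that groups five static mesh components, apparently to mark a set of item placements.
; GetAllTransform returns the world transforms of all five meshes as an array for other code to read.
; It has no other logic: the event graph holds only disabled default events and the construction script is empty.
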(event EventBeginPlay)

(event Collision|EventActorBeginOverlap
  (params (OtherActor :type Actor%20Object%20Reference)))

(event EventTick
  (params (DeltaSeconds :type Float%20%28single-precision%29)))

(fn ConstructionScript)

(fn GetAllTransform
  (return (Utilities|Array|MakeArray (Transformation|GetWorldTransform (Variables|Default|GetStaticMesh)) (Transformation|GetWorldTransform (Variables|Default|GetStaticMesh1)) (Transformation|GetWorldTransform (Variables|Default|GetStaticMesh2)) (Transformation|GetWorldTransform (Variables|Default|GetStaticMesh3)) (Transformation|GetWorldTransform (Variables|Default|GetStaticMesh4)))))